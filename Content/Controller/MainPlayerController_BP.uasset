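; Main player controller that handles input, HUD updates and the item inventory.
; Tick pushes player health, stamina and mana ratios to the HUD overlay held by TeamProjectInstance, which also toggles option and map widgets.
; Keys drive quit, interaction, item slots and Alt+1–3 partner control modes.
; Events handle floating damage numbers, health-bar visibility and clamped healing, while functions fill the first empty Inventory slot and move or swap items and icons.
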(event EventBeginPlay
  (bind _asmy_character (Utilities|Casting|CastToMyCharacter (Game|Player|GetPlayerPawn 0)))
  (Variables|Default|SetPlayerCharacter _asmy_character)
  (bind _asteam_project_instance (Utilities|Casting|CastToTeamProjectInstance (Game|GetGameInstance)))
  (Variables|Default|SetInstanceReference _asteam_project_instance))

(event EventTick
  (params (DeltaSeconds :type Float%20%28single-precision%29))
  (bind _playercharacter (Variables|Default|GetPlayerCharacter))
  (bind _asteam_project_instance (Utilities|Casting|CastToTeamProjectInstance (Game|GetGameInstance)))
  (Default|SetHealth (Variables|/ProjectUI/Game/HUD/Character/CharacterHUDOverlay.CharacterHUDOverlay_C|GetCharacterHealthBar (Variables|/Game/GameInstance/TeamProjectInstance.TeamProjectInstance_C|GetHUDOVerlay _asteam_project_instance)) (/ (Variables|/Script/TeamPlayer.MyCharacter|GetfHP _playercharacter) (Variables|/Script/TeamPlayer.MyCharacter|GetfMaxHP _playercharacter)))
  (Progress|SetPercent (Variables|/ProjectUI/Game/HUD/Character/CharacterSteminaBar.CharacterSteminaBar_C|GetSteminaBar (Variables|/ProjectUI/Game/HUD/Inventory/ActionBar.ActionBar_C|GetCharacterSteminaBar (Variables|/ProjectUI/Game/HUD/Character/CharacterHUDOverlay.CharacterHUDOverlay_C|GetActionBar (Variables|/Game/GameInstance/TeamProjectInstance.TeamProjectInstance_C|GetHUDOVerlay _asteam_project_instance)))) (/ (Variables|/Script/TeamPlayer.MyCharacter|GetfStBar _playercharacter) (Variables|/Script/TeamPlayer.MyCharacter|GetfMaxStBar _playercharacter)))
  (Progress|SetPercent (Variables|/ProjectUI/Game/HUD/Character/CharacterManaBar.CharacterManaBar_C|GetManaBar (Variables|/ProjectUI/Game/HUD/Inventory/ActionBar.ActionBar_C|GetCharacterManaBar (Variables|/ProjectUI/Game/HUD/Character/CharacterHUDOverlay.CharacterHUDOverlay_C|GetActionBar (Variables|/Game/GameInstance/TeamProjectInstance.TeamProjectInstance_C|GetHUDOVerlay _asteam_project_instance)))) (/ (Variables|/Script/TeamPlayer.MyCharacter|GetfMP _playercharacter) (Variables|/Script/TeamPlayer.MyCharacter|GetfMaxMP _playercharacter))))

(event EventUseItemHealingPoint
  (params (IncreaseHealth :type Integer))
  (bind _asbp_my_character_child (Utilities|Casting|CastToBP_MyCharacter_Child (Game|Player|GetPlayerPawn 0)))
  (Variables|/Script/TeamPlayer.MyCharacter|SetfHP _asbp_my_character_child (+ (Variables|/Script/TeamPlayer.MyCharacter|GetfHP _asbp_my_character_child) (Math|Conversions|ToFloat(Integer) IncreaseHealth)))
  (if (<= (Variables|/Script/TeamPlayer.MyCharacter|GetfMaxHP _asbp_my_character_child) (Variables|/Script/TeamPlayer.MyCharacter|GetfHP _asbp_my_character_child))
    (Variables|/Script/TeamPlayer.MyCharacter|SetfHP _asbp_my_character_child (Variables|/Script/TeamPlayer.MyCharacter|GetfMaxHP _asbp_my_character_child))))

(event EventShowHitNumber
  (params (Damage :type Integer) (HitLocation :type Vector :default "0, 0, 0"))
  ;[1 1 1] 코멘트
  (bind _returnvalue (UserInterface|CreateWidget "/ProjectUI/Game/HUD/GamePlay/HItNumber.HItNumber_C"))
  (UserInterface|Viewport|AddtoViewport _returnvalue 0)
  (Class|UserWidget|SetPositioninViewport _returnvalue (.ScreenPosition (Class|GameplayStatics|ProjectWorldtoScreen (Game|GetPlayerController 0) HitLocation false)) true)
  (Class|MainPlayerController|StoreHitNumber _returnvalue HitLocation)
  (Variables|/ProjectUI/Game/HUD/GamePlay/HItNumber.HItNumber_C|SetHitText _returnvalue (Utilities|Text|ToText(Integer) Damage))
  (UserInterface|Animation|PlayAnimation _returnvalue (Variables|/ProjectUI/Game/HUD/GamePlay/HItNumber.HItNumber_C|GetHitNumberAnimation _returnvalue) 0.0 1 "Forward" 1.0 false))

(event EventShowHealthBar
  (params (widget :type Widget%20Component%20Object%20Reference))
  (Utilities|IsValid widget
    (:Is%20Valid
      (Widget|SetVisibility (UserInterface|GetUserWidgetObject widget) "Visible")
      (|CallParentFunction widget))))

(event EventHideHealthBar
  (Widget|SetVisibility (UserInterface|GetUserWidgetObject (stale EventShowHealthBar widget)) "Hidden"))

(event Input|ActionEvents|InputActionInterect
  (params (Key :type Key%20Structure :default "None"))
  (bind _overlapitem (Variables|Default|GetOverlapItem))
  (:Pressed
    (Default|CallInteraction)
    (if (Variables|Default|GetbInterActionKey)
      (Utilities|IsValid _overlapitem
        (:Is%20Valid
          (Class|MainPlayerController|OverlapSetInventoryItems _overlapitem))))))

(event Input|ActionEvents|InputActionQuit
  (params (Key :type Key%20Structure :default "None"))
  (:Pressed
    (Default|CallQuitUI)))

(event Input|ActionEvents|InputActionAlt+1
  (params (Key :type Key%20Structure :default "None"))
  (:Pressed
    (bind _asbp_my_character (Utilities|Casting|CastToBP_MyCharacter (Variables|Default|GetPlayerCharacter)))
    (Utilities|IsValid (Variables|/TeamPlayer/Blueprints/Character/BP_MyCharacter.BP_MyCharacter_C|GetPartner _asbp_my_character)
      (:Is%20Valid
        (if (Utilities|Enum|NotEqual(Enum) (Variables|/Game/AI/NPC/PartnerNPC/Brain/BP_PartnerController.BP_PartnerController_C|GetEControlMode (Variables|/TeamPlayer/Blueprints/Character/BP_MyCharacter.BP_MyCharacter_C|GetPartner _asbp_my_character)) "EControl_Dead")
          (Default|SetControlMode (Variables|/TeamPlayer/Blueprints/Character/BP_MyCharacter.BP_MyCharacter_C|GetPartner _asbp_my_character) "EControl_Accompany"))))))

(event Input|ActionEvents|InputActionAlt+2
  (params (Key :type Key%20Structure :default "None"))
  (:Pressed
    (bind _asbp_my_character (Utilities|Casting|CastToBP_MyCharacter (Variables|Default|GetPlayerCharacter)))
    (Utilities|IsValid (Variables|/TeamPlayer/Blueprints/Character/BP_MyCharacter.BP_MyCharacter_C|GetPartner _asbp_my_character)
      (:Is%20Valid
        (if (Utilities|Enum|NotEqual(Enum) (Variables|/Game/AI/NPC/PartnerNPC/Brain/BP_PartnerController.BP_PartnerController_C|GetEControlMode (Variables|/TeamPlayer/Blueprints/Character/BP_MyCharacter.BP_MyCharacter_C|GetPartner _asbp_my_character)) "EControl_Dead")
          (Default|SetControlMode (Variables|/TeamPlayer/Blueprints/Character/BP_MyCharacter.BP_MyCharacter_C|GetPartner _asbp_my_character) "EControl_Accompnay_Aggressive"))))))

(event Input|ActionEvents|InputActionAlt+3
  (params (Key :type Key%20Structure :default "None"))
  (:Pressed
    (bind _asbp_my_character (Utilities|Casting|CastToBP_MyCharacter (Variables|Default|GetPlayerCharacter)))
    (Utilities|IsValid (Variables|/TeamPlayer/Blueprints/Character/BP_MyCharacter.BP_MyCharacter_C|GetPartner _asbp_my_character)
      (:Is%20Valid
        (if (Utilities|Enum|NotEqual(Enum) (Variables|/Game/AI/NPC/PartnerNPC/Brain/BP_PartnerController.BP_PartnerController_C|GetEControlMode (Variables|/TeamPlayer/Blueprints/Character/BP_MyCharacter.BP_MyCharacter_C|GetPartner _asbp_my_character)) "EControl_Dead")
          (Default|SetControlMode (Variables|/TeamPlayer/Blueprints/Character/BP_MyCharacter.BP_MyCharacter_C|GetPartner _asbp_my_character) "EControl_Waiting_Aggressive"))))))

(event Input|KeyboardEvents|O
  (params (Key :type Key%20Structure :default "None"))
  (:Pressed
    (bind _asteam_project_instance (Utilities|Casting|CastToTeamProjectInstance (Game|GetGameInstance)))
    (if (Variables|/Game/GameInstance/TeamProjectInstance.TeamProjectInstance_C|GetOpenOptionWidget _asteam_project_instance)
      (Default|HideinGameOption _asteam_project_instance)
      (else
        (Default|ShowinGameOption _asteam_project_instance)))))

(event Input|KeyboardEvents|3
  (params (Key :type Key%20Structure :default "None"))
  (:Pressed
    (Class|MainPlayerController|UseItem 2)))

(event Input|KeyboardEvents|2
  (params (Key :type Key%20Structure :default "None"))
  (:Pressed
    (Class|MainPlayerController|UseItem 1)))

(event Input|KeyboardEvents|4
  (params (Key :type Key%20Structure :default "None"))
  (:Pressed
    (Class|MainPlayerController|UseItem 3)))

(event Input|KeyboardEvents|5
  (params (Key :type Key%20Structure :default "None"))
  (:Pressed
    (Class|MainPlayerController|UseItem 4)))

(event Input|KeyboardEvents|6
  (params (Key :type Key%20Structure :default "None"))
  (:Pressed
    (Class|MainPlayerController|UseItem 5)))

(event Input|KeyboardEvents|7
  (params (Key :type Key%20Structure :default "None"))
  (:Pressed
    (Class|MainPlayerController|UseItem 6)))

(event Input|KeyboardEvents|8
  (params (Key :type Key%20Structure :default "None"))
  (:Pressed
    (Class|MainPlayerController|UseItem 7)))

(event Input|KeyboardEvents|9
  (params (Key :type Key%20Structure :default "None"))
  (:Pressed
    (Class|MainPlayerController|UseItem 8)))

(event Input|KeyboardEvents|M
  (params (Key :type Key%20Structure :default "None"))
  (:Pressed
    (Utilities|FlowControl|FlipFlop
      (:A
        (bind _asteam_project_instance (Utilities|Casting|CastToTeamProjectInstance (Game|GetGameInstance)))
        (Default|ShowMapWidget _asteam_project_instance))
      (:B
        (Default|HideMapWidget _asteam_project_instance)))))

(event Input|KeyboardEvents|0
  (params (Key :type Key%20Structure :default "None"))
  (:Pressed
    (Class|MainPlayerController|UseItem 9)))

(event Input|KeyboardEvents|1
  (params (Key :type Key%20Structure :default "None"))
  (:Pressed
    (Class|MainPlayerController|UseItem)))

(fn ConstructionScript)

(fn PickupItem
  (params (PickupItem :type Item%20Object%20Reference))
  (Utilities|Array|SetArrayElem (Variables|Default|GetInventory self) (CallFunction|FindEmptySlot) PickupItem)
  (bind _asgame_object (Utilities|Casting|CastToGameObject PickupItem))
  (Variables|/Script/KGCA38.Item|SetItemIcon (Utilities|Array|Get(acopy) (Variables|Default|GetInventory self) (Variables|Default|GetEmptySlot)) (Variables|/Script/KGCA38.Item|GetItemIcon _asgame_object)))

(fn FindEmptySlot
  (bind (_array_element _array_index) (Utilities|Array|ForEachLoopwithBreak (Variables|Default|GetInventory self) :!label _label)
    (:LoopBody
      (if (not (Utilities|IsValid _array_element))
        (bind _output_get (Variables|Default|SetEmptySlot _array_index))
        (goto _label Break)))
    (:Completed
      (return _output_get))))

(fn MoveItem
  (params (From :type Integer) (To :type Integer))
  (bind _self self)
  (bind _self_2 self)
  (bind _inventory (Variables|Default|GetInventory _self))
  (bind _inventory_2 (Variables|Default|GetInventory _self_2))
  (LocalVariables|SetLocalFrom From)
  (LocalVariables|SetLocalTo To)
  (if (Utilities|IsValid (Utilities|Array|Get(acopy) (Variables|Default|GetInventory self) (LocalVariables|GetLocalTo)))
    (LocalVariables|SetLocalTempObject (Utilities|Array|Get(acopy) (Variables|Default|GetInventory self) (LocalVariables|GetLocalTo)))
    (Utilities|Array|SetArrayElem _inventory (LocalVariables|GetLocalTo) (Utilities|Array|Get(acopy) _inventory (LocalVariables|GetLocalFrom)))
    (Utilities|Array|SetArrayElem (Variables|Default|GetInventory self) (LocalVariables|GetLocalFrom) (LocalVariables|GetLocalTempObject))
    (LocalVariables|SetLocalSwapping true)
    (else
      (Utilities|Array|SetArrayElem _inventory_2 (LocalVariables|GetLocalTo) (Utilities|Array|Get(acopy) _inventory_2 (LocalVariables|GetLocalFrom)))
      (Utilities|Array|SetArrayElem (Variables|Default|GetInventory self) (LocalVariables|GetLocalFrom) 0)
      (LocalVariables|SetLocalSwapping false)))
  (return (LocalVariables|GetLocalSwapping)))

(fn MoveImage
  (params (From :type Integer) (To :type Integer) (Image :type Texture%202D%20Object%20Reference) (Swapping? :type Boolean))
  (bind _self self)
  (bind _self_2 self)
  (bind _inventory (Variables|Default|GetInventory _self))
  (bind _inventory_2 (Variables|Default|GetInventory _self_2))
  (LocalVariables|SetLocalFrom From)
  (LocalVariables|SetLocalTo To)
  (LocalVariables|SetLocalImage Image)
  (if Swapping?
    (LocalVariables|SetLocalTempImage (Variables|/Script/KGCA38.Item|GetItemIcon (Utilities|Array|Get(acopy) _inventory (LocalVariables|GetLocalTo))))
    (Variables|/Script/KGCA38.Item|SetItemIcon (Utilities|Array|Get(acopy) _inventory (LocalVariables|GetLocalTo)) (LocalVariables|GetLocalImage))
    (Variables|/Script/KGCA38.Item|SetItemIcon (Utilities|Array|Get(acopy) _inventory (LocalVariables|GetLocalFrom)) (LocalVariables|GetLocalTempImage))
    (else
      (Variables|/Script/KGCA38.Item|SetItemIcon (Utilities|Array|Get(acopy) _inventory_2 (LocalVariables|GetLocalTo)) (LocalVariables|GetLocalImage))
      (Variables|/Script/KGCA38.Item|SetItemIcon (Utilities|Array|Get(acopy) _inventory_2 (LocalVariables|GetLocalFrom)) (LocalVariables|GetDefault%20Texture)))))
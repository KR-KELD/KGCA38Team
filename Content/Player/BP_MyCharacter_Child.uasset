(event EventBeginPlay
  (|CallParentFunction) ; 지금 이 노드는 비활성 상태입니다. \n핀을 끌어서 다른 노드를 연결하면 활성화됩니다.
)

(event Collision|EventActorBeginOverlap
  (params (OtherActor :type Actor%20Object%20Reference))
  (|CallParentFunction OtherActor) ; 지금 이 노드는 비활성 상태입니다. \n핀을 끌어서 다른 노드를 연결하면 활성화됩니다.
)

(event EventTick
  (params (DeltaSeconds :type Float%20%28single-precision%29))
  (|CallParentFunction DeltaSeconds) ; 지금 이 노드는 비활성 상태입니다. \n핀을 끌어서 다른 노드를 연결하면 활성화됩니다.
)

(event Input|KeyboardEvents|O
  (params (Key :type Key%20Structure :default "None"))
  (:Pressed
    (Utilities|FlowControl|FlipFlop
      (:A
        (bind _asteam_project_instance (Utilities|Casting|CastToTeamProjectInstance (Game|GetGameInstance)))
        (Default|ShowinGameOption _asteam_project_instance))
      (:B
        (Default|HideinGameOption _asteam_project_instance)))))

(event Input|KeyboardEvents|I
  (params (Key :type Key%20Structure :default "None"))
  (:Pressed
    (bind _asteam_project_instance (Utilities|Casting|CastToTeamProjectInstance (Game|GetGameInstance)))
    (if (Variables|/Game/GameInstance/TeamProjectInstance.TeamProjectInstance_C|GetOpenInventory _asteam_project_instance)
      (Default|HideInventory _asteam_project_instance)
      (else
        (Default|ShowInventory _asteam_project_instance)))))

(fn ConstructionScript
  (|CallParentFunction))
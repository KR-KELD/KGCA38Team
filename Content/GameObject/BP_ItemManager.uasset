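; BP_ItemManager is an item manager Blueprint that spawns item actors at a given transform by percentage chance.
; SpawnItem compares a random roll against the clamped percentage, then spawns the class at the requested index in the Items array.
; An invalid index falls back to a random class from that array.
; The event graph and construction script hold no logic, so spawning runs only when SpawnItem is called.
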(event EventBeginPlay)

(event Collision|EventActorBeginOverlap
  (params (OtherActor :type Actor%20Object%20Reference)))

(event EventTick
  (params (DeltaSeconds :type Float%20%28single-precision%29)))

(fn ConstructionScript)

(fn SpawnItem
  (params (ItemIndex :type Integer) (SpawnPos :type Transform) (Percentage :type Integer))
  (bind _items (Variables|Default|GetItems))
  (if (Math|Integer|InRange(Integer) (Math|Random|RandomIntegerinRange 0 100) 0 (Math|Integer|Clamp(Integer) Percentage 0 100))
    (if (Utilities|Array|IsValidIndex _items ItemIndex)
      (Game|SpawnActorfromClass (Utilities|Array|Get(acopy) _items ItemIndex) SpawnPos "Undefined" 0 0)
      (else
        (Game|SpawnActorfromClass (.OutItem (Utilities|Array|Random _items)) SpawnPos "Undefined" 0 0)))))
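; BP_Partner is the partner NPC, a sword-wielding AI character that damages enemies in melee.
; On BeginPlay it sets its stats, registers with TeamProjectInstance's AI container and binds hit and death delegates.
; AttackEnemy plays the attack montage, and weapon overlaps with EnemyCollision-tagged components apply damage, sound and blood.
; Reset, hit and death switch off weapon overlaps; nothing in this graph switches them back on.
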(event OnComponentBeginOverlap(WeaponCollider)
  (params (OverlappedComponent :type Primitive%20Component%20Object%20Reference) (OtherActor :type Actor%20Object%20Reference) (OtherComp :type Primitive%20Component%20Object%20Reference) (OtherBodyIndex :type Integer) (bFromSweep :type Boolean) (SweepResult :type Hit%20Result%20Structure%20%28by%20ref%29))
  (bind _returnvalue (Transformation|GetActorLocation OtherActor))
  (if (Components|ComponentHasTag OtherComp "EnemyCollision")
    (Game|Damage|ApplyDamage OtherActor (.Damage (Utilities|Struct|BreakCharacterDataStruct (Variables|Default|GetCharacterInfo))) 0 self)
    (Audio|PlaySoundatLocation "/TeamAI/Character/Partner/Sound/Sq_Sword_Hit.Sq_Sword_Hit" _returnvalue "0, 0, 0" 1.0 1.0 0.0 0 0 0)
    (Effects|SpawnEmitteratLocation "/TeamAI/Effect/Blood/P_Blood.P_Blood" _returnvalue)))

(event Custom|AIDeadEvent
  (params (msg :type String))
  (Variables|/Script/Engine.PrimitiveComponent|SetbGenerateOverlapEvents (Variables|Default|GetWeaponCollider) false)
  (Audio|PlaySoundatLocation "/TeamAI/Character/Partner/Sound/Sq_Partner_Dead.Sq_Partner_Dead" (Transformation|GetActorLocation) "0, 0, 0" 1.0 1.0 0.0 0 0 0))

(event Custom|AIHitEvent
  (params (actor :type Actor%20Object%20Reference))
  (Animation|PlayAnimMontage "/Game/AI/NPC/PartnerNPC/Animations/AM_Partner_Hit.AM_Partner_Hit" 1.0 "None")
  (Variables|/Script/Engine.PrimitiveComponent|SetbGenerateOverlapEvents (Variables|Default|GetWeaponCollider) false))

(event EventBeginPlay
  (Class|AIBase|AIReset)
  (bind _asteam_project_instance (Utilities|Casting|CastToTeamProjectInstance (Game|GetGameInstance)))
  (Default|SetAIContainer _asteam_project_instance (.Type (Utilities|Struct|BreakCharacterDataStruct (Variables|Default|GetCharacterInfo))) self)
  (EventDispatchers|BindEventtoHitDelegate (delegate Custom|AIHitEvent))
  (EventDispatchers|BindEventtoDeadDelegate (delegate Custom|AIDeadEvent)))

(event Collision|EventActorBeginOverlap
  (params (OtherActor :type Actor%20Object%20Reference)))

(event EventTick
  (params (DeltaSeconds :type Float%20%28single-precision%29)))

(event EventAttackEnemy
  (Animation|PlayAnimMontage "/Game/AI/NPC/PartnerNPC/Animations/AM_Partner_Attack.AM_Partner_Attack" 1.0 "None"))

(event EventAIReset
  (Variables|Default|SetCharacterInfo (Utilities|Struct|MakeCharacterDataStruct "Partner" "EPartner" 1.5e+02 1.5e+02 3e+01))
  (Variables|/Script/Engine.PrimitiveComponent|SetbGenerateOverlapEvents (Variables|Default|GetWeaponCollider) false))

(fn ConstructionScript)
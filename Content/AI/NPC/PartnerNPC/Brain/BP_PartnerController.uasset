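; AI controller for the partner NPC that accompanies or waits for the player and fights monsters according to a switchable control mode.
; Control modes write state, mode and waiting point to the Blackboard and set movement.
; Being hit outside battle switches non-aggressive modes to aggressive accompany, while perceived monsters trigger battle only in aggressive modes.
; Battle selection randomly picks boundary or trace behavior, and HUD widgets show health and mode.
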(event OnTargetPerceptionUpdated(PerceptionComponent)
  (params (Actor :type Actor%20Object%20Reference) (Stimulus :type AI%20Stimulus%20Structure))
  (if (Actor|ActorHasTag Actor "Monster")
    (if (and (Utilities|String|Contains (Variables|Default|GetControlMode) "Aggressive") (Utilities|Enum|NotEqual(Enum) (Variables|Default|GetAIState) "State_Battle"))
      (Class|MyAIController|UpdateState "State_BattleReady")
      (AI|Components|Blackboard|SetValueasObject (AI|GetBlackboard 0) (Variables|Default|GetTargetActor) Actor))))

(event Custom|AddHitEvent
  (params (actor :type Actor%20Object%20Reference))
  (bind _returnvalue (AI|GetBlackboard 0))
  (if (Utilities|Enum|NotEqual(Enum) (Variables|Default|GetAIState) "State_Battle")
    (if (Utilities|String|Contains (Variables|Default|GetControlMode) "Aggressive")
      _
      (else
        (bind _output_get (Variables|Default|SetControlMode "Control_Accompany_Aggressive"))
        (Variables|Default|SetEControlMode "EControl_Accompnay_Aggressive")
        (CallFunction|UpdateWidget)
        (Class|BlackboardComponent|SetValueasString _returnvalue (Variables|Default|GetBBControlMode) _output_get)))
    (Class|MyAIController|UpdateState "State_BattleReady")
    (AI|Components|Blackboard|SetValueasObject _returnvalue (Variables|Default|GetTargetActor) actor)))

(event Custom|WidgetEvent
  (params (actor :type Actor%20Object%20Reference))
  (CallFunction|UpdateWidget))

(event Custom|WidgetUpdate
  (params (msg :type String))
  (CallFunction|UpdateWidget))

(event EventBeginPlay)

(event EventTick
  (params (DeltaSeconds :type Float%20%28single-precision%29)))

(event EventPossess
  (params (PossessedPawn :type Pawn%20Object%20Reference))
  (bind _output_get (Variables|Default|SetAIData (Utilities|Struct|MakeAIDataStruct 1.5e+02 6e+02 1.5e+03 8e+01 1.5 1.5e+03 2e+03 6e+01 4e+02 1.0)))
  (bind _asaibase (Utilities|Casting|CastToAIBase PossessedPawn))
  (Class|AIBase|SetAIMove _asaibase (.WalkSpeed (Utilities|Struct|BreakAIDataStruct _output_get)) true)
  (Class|MyAIController|UpdatePerceptionData)
  (EventDispatchers|BindEventtoHitDelegate _asaibase (delegate Custom|AddHitEvent))
  (EventDispatchers|BindEventtoHitDelegate _asaibase (delegate Custom|WidgetEvent))
  (EventDispatchers|BindEventtoDeadDelegate _asaibase (delegate Custom|WidgetUpdate)))

(event EventSetAIState
  (params (StartState :type String))
  (if (Utilities|Enum|NotEqual(Enum) StartState "")
    (Class|MyAIController|UpdateState StartState)
    (else
      (Class|MyAIController|UpdateState "State_Idle"))))

(fn ConstructionScript)

(fn StateSelect
  (params (AIBase :type AI%20Base%20Object%20Reference))
  (return "State_Idle"))

(fn BattleSelect
  (params (AIBase :type AI%20Base%20Object%20Reference))
  (bind _aidata (Variables|Default|GetAIData))
  (bind _output_get (LocalVariables|SetStateCount (Math|Random|RandomIntegerinRange 0 100)))
  (if (< _output_get 30)
    (Class|AIBase|SetAIMove AIBase (.walkspeed _aidata) false)
    (return "Battle_Boundary")
    (elif (<= _output_get 100)
      (if (Variables|Default|GetIsAttackReady)
        (Class|AIBase|SetAIMove AIBase (.runspeed _aidata) true)
        (return "Battle_Trace")
        (else
          (return "Battle_Select")))
      (else
        (return "Battle_Select")))))

(fn ConnectPlayer
  (params (Player :type Actor%20Object%20Reference))
  (AI|Components|Blackboard|SetValueasObject (AI|GetBlackboard 0) (Utilities|Name|MakeLiteralName "PlayerActor") Player)
  (bind _asaibase (Utilities|Casting|CastToAIBase (Pawn|GetControlledPawn)))
  (Class|AIBase|SetAIMove _asaibase (.runspeed (Variables|Default|GetAIData)) true)
  (CallFunction|SetControlMode "EControl_Accompany")
  (CallFunction|SetWidget))

(fn SetControlMode
  (params (ControlMode :type EControlMode%20Enum :default "EControl_None"))
  (bind _aidata (Variables|Default|GetAIData))
  (bind _asaibase (Utilities|Casting|CastToAIBase (Pawn|GetControlledPawn)))
  (bind _output_get (Variables|Default|SetEControlMode ControlMode))
  (switch Utilities|FlowControl|Switch|SwitchonEControlMode _output_get
    (:EControl_None
      (Variables|Default|SetControlMode "Control_None")
      (Class|MyAIController|UpdateState "State_Idle" :!label _label)
      (Class|AIBase|SetAIMove _asaibase (.walkspeed _aidata) true))
    (:EControl_Accompany
      (Variables|Default|SetControlMode "Control_Accompany")
      (Class|MyAIController|UpdateState "State_Follow" :!label _label_2)
      (Class|AIBase|SetAIMove _asaibase (.runspeed _aidata) true))
    (:EControl_Accompnay_Aggressive
      (Variables|Default|SetControlMode "Control_Accompany_Aggressive")
      (goto _label_2))
    (:EControl_Waiting_Aggressive
      (Variables|Default|SetControlMode "Control_Waiting_Aggressive")
      (AI|Components|Blackboard|SetValueasVector (AI|GetBlackboard 0) (Variables|Default|GetWaitingPoint) (Transformation|GetActorLocation (Pawn|GetControlledPawn)))
      (goto _label)))
  (Class|BlackboardComponent|SetValueasString (AI|GetBlackboard 0) (Variables|Default|GetBBControlMode) (Variables|Default|GetControlMode))
  (Class|BlackboardComponent|SetValueasString (AI|GetBlackboard 0) (Variables|Default|GetBattleState) "Battle_Select")
  (Class|MyAIController|AttackReady true)
  (CallFunction|UpdateWidget))

(fn UpdateWidget
  (bind _npchealthbar (Variables|Default|GetNPCHealthBar))
  (bind _npcstate (Variables|Default|GetNPCState))
  (bind _asbp_partner (Utilities|Casting|CastToBP_Partner (Pawn|GetControlledPawn)))
  (Utilities|IsValid _npchealthbar
    (:Is%20Valid
      (Default|SetNPCHealth _npchealthbar (Math|Float|Clamp(Float) (/ (.hp (Variables|/Script/KGCA38.MainAIBase|GetCharacterInfo _asbp_partner)) (.maxhp (Variables|/Script/KGCA38.MainAIBase|GetCharacterInfo _asbp_partner))) 0.0 1e+02))
      (Utilities|IsValid _npcstate
        (:Is%20Valid
          (Default|SetCombatStateIcon _npcstate (Variables|Default|GetEControlMode)))))))

(fn SetWidget
  (bind _asteam_project_instance (Utilities|Casting|CastToTeamProjectInstance (Game|GetGameInstance)))
  (bind _output_get (Variables|Default|SetNPCHealthBar (Variables|/ProjectUI/Game/HUD/Character/CharacterHUDOverlay.CharacterHUDOverlay_C|GetNPCHealthBar (Variables|/Game/GameInstance/TeamProjectInstance.TeamProjectInstance_C|GetHUDOVerlay _asteam_project_instance))))
  (bind _output_get_2 (Variables|Default|SetNPCState (Variables|/ProjectUI/Game/HUD/NPC/NPCHealthBar.NPCHealthBar_C|GetCombatStateIcon (Variables|/ProjectUI/Game/HUD/Character/CharacterHUDOverlay.CharacterHUDOverlay_C|GetNPCHealthBar (Variables|/Game/GameInstance/TeamProjectInstance.TeamProjectInstance_C|GetHUDOVerlay _asteam_project_instance)))))
  (CallFunction|UpdateWidget)
  (Widget|SetVisibility _output_get "Visible")
  (Widget|SetVisibility _output_get_2 "Visible"))
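; Orc melee monster Blueprint that registers itself with the game instance's AI container on BeginPlay.
; AIReset sets its character stats and turns off weapon overlaps, and armor meshes follow the body via master pose.
; Attack plays a montage, and weapon overlaps with player-tagged components apply damage with axe sound and blood effect.
; Bound hit and death delegates disable weapon overlaps, playing a hit montage or death sound respectively.
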(event OnComponentBeginOverlap(WeaponCollider)
  (params (OverlappedComponent :type Primitive%20Component%20Object%20Reference) (OtherActor :type Actor%20Object%20Reference) (OtherComp :type Primitive%20Component%20Object%20Reference) (OtherBodyIndex :type Integer) (bFromSweep :type Boolean) (SweepResult :type Hit%20Result%20Structure%20%28by%20ref%29))
  (bind _returnvalue (Transformation|GetActorLocation OtherActor))
  (if (Components|ComponentHasTag OtherComp "PlayerCollision")
    (Game|Damage|ApplyDamage OtherActor (.Damage (Utilities|Struct|BreakCharacterDataStruct (Variables|Default|GetCharacterInfo))) 0 self)
    (Audio|PlaySoundatLocation "/TeamAI/Character/Orc/Sound/Sq_AxeHit.Sq_AxeHit" _returnvalue "0, 0, 0" 0.8 1.0 0.0 0 0 0)
    (Effects|SpawnEmitteratLocation "/TeamAI/Effect/Blood/P_Blood.P_Blood" _returnvalue)))

(event Custom|HitAnim
  (params (actor :type Actor%20Object%20Reference))
  (Animation|PlayAnimMontage "/Game/AI/Monster/DayMonster/Orc/Animations/MT_Orc_Hit.MT_Orc_Hit" 1.0 "None")
  (Variables|/Script/Engine.PrimitiveComponent|SetbGenerateOverlapEvents (Variables|Default|GetWeaponCollider) false))

(event Custom|Dead
  (params (msg :type String))
  (Variables|/Script/Engine.PrimitiveComponent|SetbGenerateOverlapEvents (Variables|Default|GetWeaponCollider) false)
  (Audio|PlaySoundatLocation "/TeamAI/Character/Orc/Sound/orc_dead.orc_dead" (Transformation|GetActorLocation) "0, 0, 0" 1.0 1.0 0.0 0 0 0))

(event EventBeginPlay
  (Class|AIBase|AIReset)
  (bind _asteam_project_instance (Utilities|Casting|CastToTeamProjectInstance (Game|GetGameInstance)))
  (Default|SetAIContainer _asteam_project_instance (.Type (Utilities|Struct|BreakCharacterDataStruct (Variables|Default|GetCharacterInfo))) self)
  (Class|SkinnedMeshComponent|SetMasterPoseComponent (Variables|Default|GetSK_ORC_BELLY_ARMOR) (Variables|Character|GetMesh) false)
  (EventDispatchers|BindEventtoHitDelegate (delegate Custom|HitAnim))
  (EventDispatchers|BindEventtoDeadDelegate (delegate Custom|Dead)))

(event Collision|EventActorBeginOverlap
  (params (OtherActor :type Actor%20Object%20Reference)))

(event EventTick
  (params (DeltaSeconds :type Float%20%28single-precision%29)))

(event EventAttackEnemy
  (Animation|PlayAnimMontage "/Game/AI/Monster/DayMonster/Orc/Animations/MT_Orc_Attack.MT_Orc_Attack" 1.0 "None"))

(event EventAIReset
  (Variables|Default|SetCharacterInfo (Utilities|Struct|MakeCharacterDataStruct "Orc" "EMonster" 1e+02 2e+01))
  (Variables|/Script/Engine.PrimitiveComponent|SetbGenerateOverlapEvents (Variables|Default|GetWeaponCollider) false))

(fn ConstructionScript)
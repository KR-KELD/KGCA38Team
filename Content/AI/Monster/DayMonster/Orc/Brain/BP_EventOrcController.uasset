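; BP_EventOrcController is the AI brain for an event Orc monster, overriding BattleSelect to pick its next battle state.
; When the attack is ready, it sets the AI to run speed with desired rotation and returns Battle_Trace; otherwise it stays in Battle_Select.
; The random roll gating this choice always passes, so attack readiness alone decides the state.
; BeginPlay and Tick hold no active logic.
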(event EventBeginPlay
  (|CallParentFunction) ; 지금 이 노드는 비활성 상태입니다. \n핀을 끌어서 다른 노드를 연결하면 활성화됩니다.
)

(event EventTick
  (params (DeltaSeconds :type Float%20%28single-precision%29))
  (|CallParentFunction DeltaSeconds) ; 지금 이 노드는 비활성 상태입니다. \n핀을 끌어서 다른 노드를 연결하면 활성화됩니다.
)

(fn ConstructionScript
  (|CallParentFunction))

(fn BattleSelect
  (params (AIBase :type AI%20Base%20Object%20Reference))
  (bind _output_get (LocalVariables|SetStateCount (Math|Random|RandomIntegerinRange 0 100)))
  (if (<= _output_get 100)
    (if (Variables|Default|GetIsAttackReady)
      (Class|AIBase|SetAIMove AIBase (.runspeed (Variables|Default|GetAIData)) true)
      (return "Battle_Trace")
      (else
        (return "Battle_Select")))
    (else
      (return "Battle_Select"))))
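; BP_OrcController is the AI controller for the Orc monster, managing its idle, patrol and battle states.
; On possession it sets tuning data, walk movement and perception, while SetAIState fills the state lists.
; Sensing a Player or Partner outside battle switches to BattleReady and sets the blackboard target; AddHitEvent does likewise, but its delegate binding is unconnected.
; Selection functions pick random states, adjusting speed and rotation for trace or boundary movement.
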(event OnTargetPerceptionUpdated(PerceptionComponent)
  (params (Actor :type Actor%20Object%20Reference) (Stimulus :type AI%20Stimulus%20Structure))
  (if (or (Actor|ActorHasTag Actor "Partner") (Actor|ActorHasTag Actor "Player"))
    (if (Utilities|Enum|NotEqual(Enum) (Variables|Default|GetAIState) "State_Battle")
      (Class|MyAIController|UpdateState "State_BattleReady")
      (AI|Components|Blackboard|SetValueasObject (AI|GetBlackboard 0) (Variables|Default|GetTargetActor) Actor))))

(event Custom|AddHitEvent
  (params (actor :type Actor%20Object%20Reference))
  (if (Utilities|Enum|NotEqual(Enum) (Variables|Default|GetAIState) "State_Battle")
    (Class|MyAIController|UpdateState "State_BattleReady")
    (AI|Components|Blackboard|SetValueasObject (AI|GetBlackboard 0) (Variables|Default|GetTargetActor) actor)))

(event EventBeginPlay)

(event EventTick
  (params (DeltaSeconds :type Float%20%28single-precision%29)))

(event EventPossess
  (params (PossessedPawn :type Pawn%20Object%20Reference))
  (bind _output_get (Variables|Default|SetAIData (Utilities|Struct|MakeAIDataStruct 1.5e+02 6e+02 1.5e+03 3e+02 1.0 2e+03 2.5e+03 6e+01 4e+02 1.0)))
  (bind _asaibase (Utilities|Casting|CastToAIBase PossessedPawn))
  (Class|AIBase|SetAIMove _asaibase (.WalkSpeed (Utilities|Struct|BreakAIDataStruct _output_get)) true)
  (Class|MyAIController|UpdatePerceptionData))

(event EventSetAIState
  (params (StartState :type String))
  (bind _aistatelist (Variables|Default|GetAIStateList))
  (bind _aibattlestatelist (Variables|Default|GetAIBattleStateList))
  (Utilities|Array|Add _aistatelist "State_Idle")
  (Utilities|Array|Add _aistatelist "State_Patrol")
  (Utilities|Array|Add _aibattlestatelist "Battle_Trace")
  (Utilities|Array|Add _aibattlestatelist "Battle_Boundary")
  (if (Utilities|Enum|NotEqual(Enum) StartState "")
    (Class|MyAIController|UpdateState StartState)
    (else
      (Class|MyAIController|UpdateState "State_Idle"))))

(fn ConstructionScript)

(fn StateSelect
  (params (AIBase :type AI%20Base%20Object%20Reference))
  (bind _aistatelist (Variables|Default|GetAIStateList))
  (bind _output_get (LocalVariables|SetState (Utilities|Array|Get(acopy) _aistatelist (Math|Random|RandomIntegerinRange 0 (- (Utilities|Array|Length _aistatelist) 1)))))
  (switch string _output_get
    (:State_Idle
      _)
    (:State_Patrol
      _))
  (Class|AIBase|SetAIMove AIBase (.walkspeed (Variables|Default|GetAIData)) true)
  (return _output_get))

(fn BattleSelect
  (params (AIBase :type AI%20Base%20Object%20Reference))
  (bind _aibattlestatelist (Variables|Default|GetAIBattleStateList))
  (bind _aidata (Variables|Default|GetAIData))
  (bind _output_get (LocalVariables|SetState (Utilities|Array|Get(acopy) _aibattlestatelist (Math|Random|RandomIntegerinRange 0 (- (Utilities|Array|Length _aibattlestatelist) 1)))))
  (switch string _output_get
    (:Battle_Trace
      (if (Variables|Default|GetIsAttackReady)
        (Class|AIBase|SetAIMove AIBase (.runspeed _aidata) true)
        (else
          (return _output_get))))
    (:Battle_Boundary
      (Class|AIBase|SetAIMove AIBase (.walkspeed _aidata) false)))
  (return _output_get))
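; Troll day-monster AI character that melee-attacks the player with one of two randomly chosen attack montages.
; BeginPlay sets its stats via AIReset, registers it with the game instance's AI container and binds hit and death delegates.
; Left and right attack colliders damage PlayerCollision-tagged components, spawn dust and switch off their overlaps after a hit.
; Being hit or dying also disables both colliders, playing a hit montage or death sound respectively.
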(event OnComponentBeginOverlap(LeftAttackCollider)
  (params (OverlappedComponent :type Primitive%20Component%20Object%20Reference) (OtherActor :type Actor%20Object%20Reference) (OtherComp :type Primitive%20Component%20Object%20Reference) (OtherBodyIndex :type Integer) (bFromSweep :type Boolean) (SweepResult :type Hit%20Result%20Structure%20%28by%20ref%29))
  (if (Components|ComponentHasTag OtherComp "PlayerCollision")
    (Game|Damage|ApplyDamage OtherActor (.Damage (Utilities|Struct|BreakCharacterDataStruct (Variables|Default|GetCharacterInfo))) 0 self)
    (Variables|/Script/Engine.PrimitiveComponent|SetbGenerateOverlapEvents (Variables|Default|GetLeftAttackCollider) false)
    (Effects|SpawnEmitteratLocation "/TeamEffect/Effects/AI/P_Dust.P_Dust" (Transformation|GetActorLocation OtherActor) "0, 0,90.000000" "0.300000,0.300000,0.300000")))

(event OnComponentBeginOverlap(RightAttackCollider)
  (params (OverlappedComponent :type Primitive%20Component%20Object%20Reference) (OtherActor :type Actor%20Object%20Reference) (OtherComp :type Primitive%20Component%20Object%20Reference) (OtherBodyIndex :type Integer) (bFromSweep :type Boolean) (SweepResult :type Hit%20Result%20Structure%20%28by%20ref%29))
  (if (Components|ComponentHasTag OtherComp "PlayerCollision")
    (Game|Damage|ApplyDamage OtherActor (.Damage (Utilities|Struct|BreakCharacterDataStruct (Variables|Default|GetCharacterInfo))) 0 self)
    (Variables|/Script/Engine.PrimitiveComponent|SetbGenerateOverlapEvents (Variables|Default|GetRightAttackCollider) false)
    (Effects|SpawnEmitteratLocation "/TeamEffect/Effects/AI/P_Dust.P_Dust" (Transformation|GetActorLocation OtherActor) "0, 0,90.000000" "0.300000,0.300000,0.300000")))

(event Custom|HitAnim
  (params (actor :type Actor%20Object%20Reference))
  (Animation|PlayAnimMontage "/Game/AI/Monster/DayMonster/Troll/Animaions/AM_Troll_Hit.AM_Troll_Hit" 1.0 "None")
  (Variables|/Script/Engine.PrimitiveComponent|SetbGenerateOverlapEvents (Variables|Default|GetRightAttackCollider) false)
  (Variables|/Script/Engine.PrimitiveComponent|SetbGenerateOverlapEvents (Variables|Default|GetLeftAttackCollider) false))

(event Custom|Dead
  (params (msg :type String))
  (Variables|/Script/Engine.PrimitiveComponent|SetbGenerateOverlapEvents (Variables|Default|GetRightAttackCollider) false)
  (Variables|/Script/Engine.PrimitiveComponent|SetbGenerateOverlapEvents (Variables|Default|GetLeftAttackCollider) false)
  (Audio|PlaySoundatLocation "/TeamAI/Character/Cyclops/Sound/Sq_Cyclops_Dead.Sq_Cyclops_Dead" (Transformation|GetActorLocation) "0, 0, 0" 1.0 1.5 0.0 0 0 0))

(event EventBeginPlay
  (Class|AIBase|AIReset)
  (bind _asteam_project_instance (Utilities|Casting|CastToTeamProjectInstance (Game|GetGameInstance)))
  (Default|SetAIContainer _asteam_project_instance (.Type (Utilities|Struct|BreakCharacterDataStruct (Variables|Default|GetCharacterInfo))) self)
  (EventDispatchers|BindEventtoHitDelegate (delegate Custom|HitAnim))
  (EventDispatchers|BindEventtoDeadDelegate (delegate Custom|Dead)))

(event Collision|EventActorBeginOverlap
  (params (OtherActor :type Actor%20Object%20Reference)))

(event EventTick
  (params (DeltaSeconds :type Float%20%28single-precision%29)))

(event EventAttackEnemy
  (switch int (Math|Random|RandomIntegerinRange 0 1)
    (:0
      (Animation|PlayAnimMontage "/Game/AI/Monster/DayMonster/Troll/Animaions/AM_Troll_Attack.AM_Troll_Attack" 1.0 "Attack1"))
    (:1
      (Animation|PlayAnimMontage "/Game/AI/Monster/DayMonster/Troll/Animaions/AM_Troll_Attack.AM_Troll_Attack" 1.0 "Attack2"))))

(event EventAIReset
  (Variables|Default|SetCharacterInfo (Utilities|Struct|MakeCharacterDataStruct "Troll" "EMonster" 2.5e+02 2.5e+02 35.0))
  (Variables|/Script/Engine.PrimitiveComponent|SetbGenerateOverlapEvents (Variables|Default|GetRightAttackCollider) false)
  (Variables|/Script/Engine.PrimitiveComponent|SetbGenerateOverlapEvents (Variables|Default|GetLeftAttackCollider) false))

(fn ConstructionScript)
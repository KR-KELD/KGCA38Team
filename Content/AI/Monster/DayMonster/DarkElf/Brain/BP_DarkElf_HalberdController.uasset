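; AI controller for the halberd-wielding Dark Elf day monster, driving its idle, patrol and battle behavior.
; On possess it sets tuning data, move speed and perception, starts in idle and runs the brain logic.
; Perceiving or being hit by a Player or Partner outside battle switches to BattleReady and stores the blackboard target.
; StateSelect and BattleSelect randomly pick the next state and adjust movement, allowing trace only when an attack is ready.
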(event OnTargetPerceptionUpdated(PerceptionComponent)
  (params (Actor :type Actor%20Object%20Reference) (Stimulus :type AI%20Stimulus%20Structure))
  (if (or (Actor|ActorHasTag Actor "Partner") (Actor|ActorHasTag Actor "Player"))
    (if (Utilities|Enum|NotEqual(Enum) (Variables|Default|GetAIState) "State_Battle")
      (Class|MyAIController|UpdateState "State_BattleReady")
      (AI|Components|Blackboard|SetValueasObject (AI|GetBlackboard 0) (Variables|Default|GetTargetActor) Actor))))

(event Custom|AddHitEvent
  (params (actor :type Actor%20Object%20Reference))
  (if (or (Actor|ActorHasTag actor "Partner") (Actor|ActorHasTag actor "Player"))
    (if (Utilities|Enum|NotEqual(Enum) (Variables|Default|GetAIState) "State_Battle")
      (Class|MyAIController|UpdateState "State_BattleReady")
      (AI|Components|Blackboard|SetValueasObject (AI|GetBlackboard 0) (Variables|Default|GetTargetActor) actor))))

(event EventBeginPlay)

(event EventTick
  (params (DeltaSeconds :type Float%20%28single-precision%29)))

(event EventPossess
  (params (PossessedPawn :type Pawn%20Object%20Reference))
  (bind _output_get (Variables|Default|SetAIData (Utilities|Struct|MakeAIDataStruct 125.0 5e+02 1.5e+03 1.1e+02 1.5 2e+03 2.5e+03 6e+01 4e+02 1.0)))
  (bind _asaibase (Utilities|Casting|CastToAIBase PossessedPawn))
  (Class|AIBase|SetAIMove _asaibase (.WalkSpeed (Utilities|Struct|BreakAIDataStruct _output_get)) true)
  (Class|MyAIController|UpdatePerceptionData)
  (EventDispatchers|BindEventtoHitDelegate _asaibase (delegate Custom|AddHitEvent))
  (Class|MyAIController|SetAIState "State_Idle")
  (AI|Logic|StartLogic (Variables|Default|GetBrainComponent)))

(event EventSetAIState
  (params (StartState :type String))
  (if (Utilities|Enum|NotEqual(Enum) StartState "")
    (Class|MyAIController|UpdateState StartState)
    (else
      (Class|MyAIController|UpdateState "State_Idle"))))

(fn ConstructionScript)

(fn BattleSelect
  (params (AIBase :type AI%20Base%20Object%20Reference))
  (bind _aidata (Variables|Default|GetAIData))
  (bind _output_get (LocalVariables|SetStateCount (Math|Random|RandomIntegerinRange 0 100)))
  (if (< _output_get 30)
    (Class|AIBase|SetAIMove AIBase (.walkspeed _aidata) false)
    (return "Battle_Boundary")
    (elif (<= _output_get 100)
      (if (Variables|Default|GetIsAttackReady)
        (Class|AIBase|SetAIMove AIBase (.runspeed _aidata) true)
        (return "Battle_Trace")
        (else
          (return "Battle_Select")))
      (else
        (return "Battle_Select")))))

(fn StateSelect
  (params (AIBase :type AI%20Base%20Object%20Reference))
  (bind _aidata (Variables|Default|GetAIData))
  (bind _output_get (LocalVariables|SetStateCount (Math|Random|RandomIntegerinRange 0 100)))
  (if (< _output_get 50)
    (Class|AIBase|SetAIMove AIBase (.walkspeed _aidata) true)
    (return "State_Idle")
    (elif (<= _output_get 100)
      (Class|AIBase|SetAIMove AIBase (.walkspeed _aidata) true)
      (return "State_Patrol")
      (else
        (return "State_Select")))))
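; BP_Arrow is the DarkElf day monster's arrow, which damages the player on hit.
; When HitCollider overlaps a component tagged PlayerCollision, it applies the stored Damage to that actor, with itself as causer.
; It then plays a bow hit sound, spawns a blood emitter at its location and destroys itself.
; The Damage value can be assigned through SetDamage, and the graphs contain no movement logic.
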(event OnComponentBeginOverlap(HitCollider)
  (params (OverlappedComponent :type Primitive%20Component%20Object%20Reference) (OtherActor :type Actor%20Object%20Reference) (OtherComp :type Primitive%20Component%20Object%20Reference) (OtherBodyIndex :type Integer) (bFromSweep :type Boolean) (SweepResult :type Hit%20Result%20Structure%20%28by%20ref%29))
  (bind _returnvalue (Transformation|GetActorLocation))
  (if (Components|ComponentHasTag OtherComp "PlayerCollision")
    (Game|Damage|ApplyDamage OtherActor (Variables|Default|GetDamage) 0 self)
    (Audio|PlaySoundatLocation "/TeamAI/Character/DarkElf/Sound/Bow/Sq_Bow_Hit.Sq_Bow_Hit" _returnvalue "0, 0, 0" 0.8 1.0 0.0 0 0 0)
    (Effects|SpawnEmitteratLocation "/TeamAI/Effect/Blood/P_Blood.P_Blood" _returnvalue)
    (Actor|SetLifeSpan 0.0)
    (Actor|DestroyActor)))

(event Collision|EventActorBeginOverlap
  (params (OtherActor :type Actor%20Object%20Reference)))

(event EventTick
  (params (DeltaSeconds :type Float%20%28single-precision%29)))

(event EventBeginPlay)

(fn ConstructionScript)

(fn SetDamage
  (params (damage :type Float%20%28single-precision%29))
  (Variables|Default|SetDamage damage))
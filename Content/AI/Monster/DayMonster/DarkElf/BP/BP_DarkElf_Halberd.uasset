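; Halberd-wielding Dark Elf enemy that sets its stats on reset and registers with the game instance's AI container.
; AttackEnemy plays the attack montage; the weapon collider damages player-tagged components, then disables its overlaps until re-enabled outside this graph.
; Bound hit and death delegates also disable the weapon.
; Hits play a reaction and briefly show the health bar, while death plays a sound and requests a chance-based item drop.
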(event OnComponentBeginOverlap(WeaponCollider)
  (params (OverlappedComponent :type Primitive%20Component%20Object%20Reference) (OtherActor :type Actor%20Object%20Reference) (OtherComp :type Primitive%20Component%20Object%20Reference) (OtherBodyIndex :type Integer) (bFromSweep :type Boolean) (SweepResult :type Hit%20Result%20Structure%20%28by%20ref%29))
  (bind _returnvalue (Transformation|GetActorLocation OtherActor))
  (if (Components|ComponentHasTag OtherComp "PlayerCollision")
    (Game|Damage|ApplyDamage OtherActor (.Damage (Utilities|Struct|BreakCharacterDataStruct (Variables|Default|GetCharacterInfo))) 0 self)
    (Variables|/Script/Engine.PrimitiveComponent|SetbGenerateOverlapEvents (Variables|Default|GetWeaponCollider) false)
    (Audio|PlaySoundatLocation "/TeamAI/Character/Partner/Sound/Sq_Sword_Hit.Sq_Sword_Hit" _returnvalue "0, 0, 0" 0.8 1.0 0.0 0 0 0)
    (Effects|SpawnEmitteratLocation "/TeamAI/Effect/Blood/P_Blood.P_Blood" _returnvalue)))

(event Custom|HitAnim
  (params (actor :type Actor%20Object%20Reference))
  (Animation|PlayAnimMontage "/Game/AI/Monster/DayMonster/DarkElf/Animations/AM_DarkElf_Halberd_Hit.AM_DarkElf_Halberd_Hit" 1.0 "None")
  (Variables|/Script/Engine.PrimitiveComponent|SetbGenerateOverlapEvents (Variables|Default|GetWeaponCollider) false)
  (Widget|SetVisibility (UserInterface|GetUserWidgetObject (Variables|Default|GetHealthBar)) "Visible")
  (bind _returnvalue (Utilities|Time|SetTimerbyEvent (delegate Custom|HideHealthBar) 4.0))
  (Variables|Default|SetHealthBarTimer _returnvalue))

(event Custom|Dead
  (params (msg :type String))
  (Audio|PlaySoundatLocation "/TeamAI/Character/DarkElf/Sound/Sq_DarkElf_Dead.Sq_DarkElf_Dead" (Transformation|GetActorLocation) "0, 0, 0" 1.0 1.0 0.0 0 0 0)
  (Variables|/Script/Engine.PrimitiveComponent|SetbGenerateOverlapEvents (Variables|Default|GetWeaponCollider) false)
  (bind _asteam_project_instance (Utilities|Casting|CastToTeamProjectInstance (Game|GetGameInstance)))
  (Default|SpawnItem (Variables|/Game/GameInstance/TeamProjectInstance.TeamProjectInstance_C|GetItemMgr _asteam_project_instance) 0 (Math|Conversions|ToTransform(Vector) (Transformation|GetActorLocation)) 40)
  (Widget|SetVisibility (UserInterface|GetUserWidgetObject (Variables|Default|GetHealthBar)) "Hidden"))

(event Custom|HideHealthBar
  (Widget|SetVisibility (UserInterface|GetUserWidgetObject (Variables|Default|GetHealthBar)) "Hidden"))

(event EventBeginPlay
  (bind _healthbar (Variables|Default|GetHealthBar))
  (bind _returnvalue (UserInterface|GetUserWidgetObject _healthbar))
  (bind _asenemy_health_bar (Utilities|Casting|CastToEnemyHealthBar _returnvalue))
  (Widget|SetVisibility _returnvalue "Hidden")
  (Variables|/ProjectUI/Game/HUD/NPC/EnemyHealthBar.EnemyHealthBar_C|SetEnemy _asenemy_health_bar self)
  (|CallParentFunction)
  (Class|AIBase|AIReset)
  (bind _asteam_project_instance (Utilities|Casting|CastToTeamProjectInstance (Game|GetGameInstance)))
  (Default|SetAIContainer _asteam_project_instance (.Type (Utilities|Struct|BreakCharacterDataStruct (Variables|Default|GetCharacterInfo))) self)
  (EventDispatchers|BindEventtoHitDelegate (delegate Custom|HitAnim))
  (EventDispatchers|BindEventtoDeadDelegate (delegate Custom|Dead)))

(event Collision|EventActorBeginOverlap
  (params (OtherActor :type Actor%20Object%20Reference))
  (|CallParentFunction OtherActor) ; 지금 이 노드는 비활성 상태입니다. \n핀을 끌어서 다른 노드를 연결하면 활성화됩니다.
)

(event EventTick
  (params (DeltaSeconds :type Float%20%28single-precision%29))
  (|CallParentFunction DeltaSeconds) ; 지금 이 노드는 비활성 상태입니다. \n핀을 끌어서 다른 노드를 연결하면 활성화됩니다.
)

(event EventAttackEnemy
  (params (EnemyActor :type Actor%20Object%20Reference))
  (Animation|PlayAnimMontage "/Game/AI/Monster/DayMonster/DarkElf/Animations/AM_DarkElf_Halberd_Attack.AM_DarkElf_Halberd_Attack" 1.0 "None"))

(event EventAIReset
  (Variables|Default|SetCharacterInfo (Utilities|Struct|MakeCharacterDataStruct "DarkElf_Halberd" "EMonster" 1.5e+02 1.5e+02 3e+01))
  (Variables|/Script/Engine.PrimitiveComponent|SetbGenerateOverlapEvents (Variables|Default|GetWeaponCollider) false))

(fn ConstructionScript
  (|CallParentFunction))
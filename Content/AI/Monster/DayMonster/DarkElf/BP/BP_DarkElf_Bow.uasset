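; BP_DarkElf_Bow is a Dark Elf archer monster AI character that attacks enemies with arrows.
; On BeginPlay it sets its character info, registers in the game instance's AI container, and binds hit and death delegates to a montage and a sound.
; AttackEnemy stores the target's location and plays the attack montage.
; A separate LunchArrow function spawns BP_Arrow from the bow socket toward that stored location, setting damage and velocity.
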(event Custom|HitAnim
  (params (actor :type Actor%20Object%20Reference))
  (Animation|PlayAnimMontage "/Game/AI/Monster/DayMonster/DarkElf/Animations/AM_DarkElf_Bow_Hit.AM_DarkElf_Bow_Hit" 1.0 "None"))

(event Custom|Dead
  (params (msg :type String))
  (Audio|PlaySoundatLocation "/TeamAI/Character/DarkElf/Sound/Sq_DarkElf_Dead.Sq_DarkElf_Dead" (Transformation|GetActorLocation) "0, 0, 0" 1.0 1.0 0.0 0 0 0))

(event EventBeginPlay
  (|CallParentFunction)
  (Class|AIBase|AIReset)
  (bind _asteam_project_instance (Utilities|Casting|CastToTeamProjectInstance (Game|GetGameInstance)))
  (Default|SetAIContainer _asteam_project_instance (.Type (Utilities|Struct|BreakCharacterDataStruct (Variables|Default|GetCharacterInfo))) self)
  (EventDispatchers|BindEventtoHitDelegate (delegate Custom|HitAnim))
  (EventDispatchers|BindEventtoDeadDelegate (delegate Custom|Dead)))

(event Collision|EventActorBeginOverlap
  (params (OtherActor :type Actor%20Object%20Reference))
  (|CallParentFunction OtherActor) ; 지금 이 노드는 비활성 상태입니다. \n핀을 끌어서 다른 노드를 연결하면 활성화됩니다.
)

(event EventTick
  (params (DeltaSeconds :type Float%20%28single-precision%29))
  (|CallParentFunction DeltaSeconds) ; 지금 이 노드는 비활성 상태입니다. \n핀을 끌어서 다른 노드를 연결하면 활성화됩니다.
)

(event EventAttackEnemy
  (params (EnemyActor :type Actor%20Object%20Reference))
  (Variables|Default|SetTargetLocation (Transformation|GetActorLocation EnemyActor))
  (Animation|PlayAnimMontage "/Game/AI/Monster/DayMonster/DarkElf/Animations/AM_DarkElf_Bow_Attack.AM_DarkElf_Bow_Attack" 1.0 "None"))

(event EventAIReset
  (Variables|Default|SetCharacterInfo (Utilities|Struct|MakeCharacterDataStruct "DarkElf_Bow" "EMonster" 1.5e+02 1.5e+02 25.0)))

(fn ConstructionScript
  (|CallParentFunction))

(fn LunchArrow
  (bind _self self)
  (bind _returnvalue (Game|SpawnActorfromClass "/Game/AI/Monster/DayMonster/DarkElf/BP/BP_Arrow.BP_Arrow_C" (Math|Transform|MakeTransform (Transformation|GetSocketLocation (Variables|Default|GetSK_DarkElf_Bow) "ArrowStart") (Math|Rotator|FindLookatRotation (Transformation|GetActorLocation) (Variables|Default|GetTargetLocation))) "AlwaysSpawn" _self _self))
  (Default|SetDamage _returnvalue (.damage (Variables|Default|GetCharacterInfo)))
  (Game|Components|ProjectileMovement|SetVelocityinLocalSpace (Variables|/Game/AI/Monster/DayMonster/DarkElf/BP/BP_Arrow.BP_Arrow_C|GetProjectileMovement _returnvalue) "3000.000000, 0, 0"))
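; Goblin monster character that fights with a melee weapon, registers itself in the game instance's AI container and uses master pose for its shoulder pad.
; AttackEnemy alternates two montage sections, and weapon overlaps with player-tagged components apply damage, blood and sound.
; Bound hit and death handlers switch off weapon overlaps; hits play a reaction montage, while death plays a sound and requests a chance-based item drop through the item manager.
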(event OnComponentBeginOverlap(WeaponCollider)
  (params (OverlappedComponent :type Primitive%20Component%20Object%20Reference) (OtherActor :type Actor%20Object%20Reference) (OtherComp :type Primitive%20Component%20Object%20Reference) (OtherBodyIndex :type Integer) (bFromSweep :type Boolean) (SweepResult :type Hit%20Result%20Structure%20%28by%20ref%29))
  (bind _returnvalue (Transformation|GetActorLocation OtherActor))
  (if (Components|ComponentHasTag OtherComp "PlayerCollision")
    (Game|Damage|ApplyDamage OtherActor (.Damage (Utilities|Struct|BreakCharacterDataStruct (Variables|Default|GetCharacterInfo))) 0 self)
    (Audio|PlaySoundatLocation "/TeamAI/Character/Partner/Sound/Sq_Sword_Hit.Sq_Sword_Hit" _returnvalue "0, 0, 0" 0.8 1.0 0.0 0 0 0)
    (Effects|SpawnEmitteratLocation "/TeamAI/Effect/Blood/P_Blood.P_Blood" _returnvalue)))

(event Custom|HitAnim
  (params (actor :type Actor%20Object%20Reference))
  (Animation|PlayAnimMontage "/Game/AI/Monster/DayMonster/Goblin/Animations/AM_Goblin_Hit.AM_Goblin_Hit" 1.0 "None")
  (Variables|/Script/Engine.PrimitiveComponent|SetbGenerateOverlapEvents (Variables|Default|GetWeaponCollider) false))

(event Custom|Dead
  (params (msg :type String))
  (Variables|/Script/Engine.PrimitiveComponent|SetbGenerateOverlapEvents (Variables|Default|GetWeaponCollider) false)
  (Audio|PlaySoundatLocation "/TeamAI/Character/Goblin/Sound/Sq_Goblin_Dead.Sq_Goblin_Dead" (Transformation|GetActorLocation) "0, 0, 0" 1.0 1.0 0.0 0 0 0)
  (bind _asteam_project_instance (Utilities|Casting|CastToTeamProjectInstance (Game|GetGameInstance)))
  (Default|SpawnItem (Variables|/Game/GameInstance/TeamProjectInstance.TeamProjectInstance_C|GetItemMgr _asteam_project_instance) 0 (Math|Conversions|ToTransform(Vector) (Transformation|GetActorLocation)) 40))

(event EventBeginPlay
  (Class|AIBase|AIReset)
  (bind _asteam_project_instance (Utilities|Casting|CastToTeamProjectInstance (Game|GetGameInstance)))
  (Default|SetAIContainer _asteam_project_instance (.Type (Utilities|Struct|BreakCharacterDataStruct (Variables|Default|GetCharacterInfo))) self)
  (Class|SkinnedMeshComponent|SetMasterPoseComponent (Variables|Default|GetSK_GOBLIN_SHOULDER_PAD) (Variables|Character|GetMesh) false)
  (EventDispatchers|BindEventtoHitDelegate (delegate Custom|HitAnim))
  (EventDispatchers|BindEventtoDeadDelegate (delegate Custom|Dead)))

(event Collision|EventActorBeginOverlap
  (params (OtherActor :type Actor%20Object%20Reference)))

(event EventTick
  (params (DeltaSeconds :type Float%20%28single-precision%29)))

(event EventAttackEnemy
  (Utilities|FlowControl|FlipFlop
    (:A
      (Animation|PlayAnimMontage "/Game/AI/Monster/DayMonster/Goblin/Animations/AM_Goblin_Attack.AM_Goblin_Attack" 1.0 "Attack01"))
    (:B
      (Animation|PlayAnimMontage "/Game/AI/Monster/DayMonster/Goblin/Animations/AM_Goblin_Attack.AM_Goblin_Attack" 1.0 "Attack02"))))

(event EventAIReset
  (Variables|Default|SetCharacterInfo (Utilities|Struct|MakeCharacterDataStruct "Goblin" "EMonster" 1e+02 1e+01))
  (Variables|/Script/Engine.PrimitiveComponent|SetbGenerateOverlapEvents (Variables|Default|GetWeaponCollider) false))

(fn ConstructionScript)
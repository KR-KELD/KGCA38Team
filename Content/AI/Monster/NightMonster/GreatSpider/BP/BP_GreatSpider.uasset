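; Enemy monster character for the Great Spider, a night monster with its own health and damage info and a melee attack.
; On BeginPlay it resets that info, registers itself in the TeamProjectInstance AI container and binds hit and death delegates.
; AttackEnemy plays the attack montage, and the attack collider damages anything tagged PlayerCollision on overlap.
; Hit and death switch that collider's overlaps off, playing a hit montage or death sound respectively.
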(event OnComponentBeginOverlap(AttackCollider)
  (params (OverlappedComponent :type Primitive%20Component%20Object%20Reference) (OtherActor :type Actor%20Object%20Reference) (OtherComp :type Primitive%20Component%20Object%20Reference) (OtherBodyIndex :type Integer) (bFromSweep :type Boolean) (SweepResult :type Hit%20Result%20Structure%20%28by%20ref%29))
  (if (Components|ComponentHasTag OtherComp "PlayerCollision")
    (Game|Damage|ApplyDamage OtherActor (.Damage (Utilities|Struct|BreakCharacterDataStruct (Variables|Default|GetCharacterInfo))) 0 self)))

(event Custom|HitAnim
  (params (actor :type Actor%20Object%20Reference))
  (Animation|PlayAnimMontage "/Game/AI/Monster/NightMonster/GreatSpider/Animations/AM_GreatSpider_Hit.AM_GreatSpider_Hit" 1.0 "None")
  (Variables|/Script/Engine.PrimitiveComponent|SetbGenerateOverlapEvents (Variables|Default|GetAttackCollider) false))

(event Custom|Dead
  (params (msg :type String))
  (Variables|/Script/Engine.PrimitiveComponent|SetbGenerateOverlapEvents (Variables|Default|GetAttackCollider) false)
  (Audio|PlaySoundatLocation "/TeamAI/Character/Spider/Sound/SQ_GS_Dead.SQ_GS_Dead" (Transformation|GetActorLocation) "0, 0, 0" 1.0 1.0 0.0 0 0 0))

(event EventBeginPlay
  (Class|AIBase|AIReset)
  (bind _asteam_project_instance (Utilities|Casting|CastToTeamProjectInstance (Game|GetGameInstance)))
  (Default|SetAIContainer _asteam_project_instance (.Type (Utilities|Struct|BreakCharacterDataStruct (Variables|Default|GetCharacterInfo))) self)
  (EventDispatchers|BindEventtoHitDelegate (delegate Custom|HitAnim))
  (EventDispatchers|BindEventtoDeadDelegate (delegate Custom|Dead)))

(event Collision|EventActorBeginOverlap
  (params (OtherActor :type Actor%20Object%20Reference)))

(event EventTick
  (params (DeltaSeconds :type Float%20%28single-precision%29)))

(event EventAttackEnemy
  (Animation|PlayAnimMontage "/Game/AI/Monster/NightMonster/GreatSpider/Animations/AM_GreatSpider_Attack.AM_GreatSpider_Attack" 1.0 "None"))

(event EventAIReset
  (Variables|Default|SetCharacterInfo (Utilities|Struct|MakeCharacterDataStruct "GreatSpider" "EMonster" 2e+02 5e+01))
  (Variables|/Script/Engine.PrimitiveComponent|SetbGenerateOverlapEvents (Variables|Default|GetAttackCollider) false))

(fn ConstructionScript)
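; AI controller for the Cyclops night monster that chooses its states and reacts to threats.
; On possess it loads tuning data, sets walk movement, updates perception and binds the pawn's hit delegate.
; Hits, or perceiving Player- or Partner-tagged actors, switch it to BattleReady and set the blackboard target unless already in battle.
; StateSelect randomly picks idle or patrol at walk speed; BattleSelect picks from a trace-only list, running when attack is ready.
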(event OnTargetPerceptionUpdated(PerceptionComponent)
  (params (Actor :type Actor%20Object%20Reference) (Stimulus :type AI%20Stimulus%20Structure))
  (if (or (Actor|ActorHasTag Actor "Partner") (Actor|ActorHasTag Actor "Player"))
    (if (Utilities|Enum|NotEqual(Enum) (Variables|Default|GetAIState) "State_Battle")
      (Class|MyAIController|UpdateState "State_BattleReady")
      (AI|Components|Blackboard|SetValueasObject (AI|GetBlackboard 0) (Variables|Default|GetTargetActor) Actor))))

(event Custom|AddHitEvent
  (params (actor :type Actor%20Object%20Reference))
  (if (Utilities|Enum|NotEqual(Enum) (Variables|Default|GetAIState) "State_Battle")
    (Class|MyAIController|UpdateState "State_BattleReady")
    (AI|Components|Blackboard|SetValueasObject (AI|GetBlackboard 0) (Variables|Default|GetTargetActor) actor)))

(event EventBeginPlay)

(event EventTick
  (params (DeltaSeconds :type Float%20%28single-precision%29)))

(event EventPossess
  (params (PossessedPawn :type Pawn%20Object%20Reference))
  (bind _output_get (Variables|Default|SetAIData (Utilities|Struct|MakeAIDataStruct 4e+02 4e+02 1.5e+03 4e+02 1.5 3e+03 3.5e+03 6e+01 4e+02 1.0)))
  (bind _asaibase (Utilities|Casting|CastToAIBase PossessedPawn))
  (Class|AIBase|SetAIMove _asaibase (.WalkSpeed (Utilities|Struct|BreakAIDataStruct _output_get)) true)
  (Class|MyAIController|UpdatePerceptionData)
  (EventDispatchers|BindEventtoHitDelegate _asaibase (delegate Custom|AddHitEvent)))

(event EventSetAIState
  (params (StartState :type String))
  (bind _aistatelist (Variables|Default|GetAIStateList))
  (Utilities|Array|Add _aistatelist "State_Idle")
  (Utilities|Array|Add _aistatelist "State_Patrol")
  (Utilities|Array|Add (Variables|Default|GetAIBattleStateList) "Battle_Trace")
  (if (Utilities|Enum|NotEqual(Enum) StartState "")
    (Class|MyAIController|UpdateState StartState)
    (else
      (Class|MyAIController|UpdateState "State_Idle"))))

(fn ConstructionScript)

(fn BattleSelect
  (params (AIBase :type AI%20Base%20Object%20Reference))
  (bind _output_get (LocalVariables|SetState (.OutItem (Utilities|Array|Random (Variables|Default|GetAIBattleStateList)))))
  (switch string _output_get
    (:Battle_Trace
      (if (Variables|Default|GetIsAttackReady)
        (Class|AIBase|SetAIMove AIBase (.runspeed (Variables|Default|GetAIData)) true)
        (return _output_get)
        (else
          (return _output_get))))))

(fn StateSelect
  (params (AIBase :type AI%20Base%20Object%20Reference))
  (bind _output_get (LocalVariables|SetState (.OutItem (Utilities|Array|Random (Variables|Default|GetAIStateList)))))
  (switch string _output_get
    (:State_Idle
      _)
    (:State_Patrol
      _))
  (Class|AIBase|SetAIMove AIBase (.walkspeed (Variables|Default|GetAIData)) true)
  (return _output_get))
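; BP_Orc is a day monster NPC orc that attacks the player with a melee weapon.
; On BeginPlay it sets its monster stats, registers with the game instance's AI container and slaves its armor meshes to the body via master pose.
; Hit and death delegates switch off the weapon collider, with hits also playing a montage.
; AttackEnemy plays the attack montage, while weapon overlaps damage components tagged PlayerCollision.
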(event OnComponentBeginOverlap(WeaponCollider)
  (params (OverlappedComponent :type Primitive%20Component%20Object%20Reference) (OtherActor :type Actor%20Object%20Reference) (OtherComp :type Primitive%20Component%20Object%20Reference) (OtherBodyIndex :type Integer) (bFromSweep :type Boolean) (SweepResult :type Hit%20Result%20Structure%20%28by%20ref%29))
  (if (Components|ComponentHasTag OtherComp "PlayerCollision")
    (Game|Damage|ApplyDamage OtherActor (.Damage (Utilities|Struct|BreakCharacterDataStruct (Variables|Default|GetCharacterInfo))) 0 self)))

(event Custom|HitAnim
  (params (msg :type String))
  (Animation|PlayAnimMontage "/TeamAI/Character/Orc/Animations/MT_Hit.MT_Hit" 1.0 "None")
  (Components|Activation|Deactivate (Variables|Default|GetWeaponCollider)))

(event Custom|DeadEvent
  (params (msg :type String))
  (Components|Activation|Deactivate (Variables|Default|GetWeaponCollider)))

(event EventBeginPlay
  (bind _output_get (Variables|Default|SetCharacterInfo (Utilities|Struct|MakeCharacterDataStruct "EMonster" 1e+02 2e+01)))
  (bind _asteam_project_instance (Utilities|Casting|CastToTeamProjectInstance (Game|GetGameInstance)))
  (bind _containercode (Default|SetAIContainer _asteam_project_instance (.Type (Utilities|Struct|BreakCharacterDataStruct _output_get)) self))
  (Variables|Default|SetCode _containercode)
  (Class|SkinnedMeshComponent|SetMasterPoseComponent (Variables|Default|GetSK_ORC_BELLY_ARMOR) (Variables|Character|GetMesh) false)
  (EventDispatchers|BindEventtoHitDelegate (delegate Custom|HitAnim))
  (EventDispatchers|BindEventtoDeadDelegate (delegate Custom|DeadEvent))
  (Components|Activation|Deactivate (Variables|Default|GetWeaponCollider)))

(event Collision|EventActorBeginOverlap
  (params (OtherActor :type Actor%20Object%20Reference)))

(event EventTick
  (params (DeltaSeconds :type Float%20%28single-precision%29)))

(event EventAttackEnemy
  (Animation|PlayAnimMontage "/TeamAI/Character/Orc/Animations/MT_Attack.MT_Attack" 1.0 "None"))

(fn ConstructionScript)
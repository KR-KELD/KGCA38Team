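; BP_BattleRoomActor is an ambush room that fills itself with orcs and turns them on the player.
; On BeginPlay it tries repeatedly to spawn BP_EventOrc at random navigable points nearby, storing them in MonsterContainer.
; The first Box overlap consumes the one-shot trap, even if the player cast fails.
; For a player, each orc's AI controller gets overridden AI data, battle-ready state without Battle_Boundary, the player as TargetActor, and started logic.
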(event OnComponentBeginOverlap(Box)
  (params (OverlappedComponent :type Primitive%20Component%20Object%20Reference) (OtherActor :type Actor%20Object%20Reference) (OtherComp :type Primitive%20Component%20Object%20Reference) (OtherBodyIndex :type Integer) (bFromSweep :type Boolean) (SweepResult :type Hit%20Result%20Structure%20%28by%20ref%29))
  (CallFunction|TraponPlayer OtherActor))

(event EventBeginPlay
  (for _index (range 0 15)
    (bind (_randomlocation _returnvalue) (Class|NavigationSystemV1|GetRandomLocationinNavigableRadius (Transformation|GetActorLocation) 1.5e+03 0 0))
    (if _returnvalue
      (bind _returnvalue_2 (Game|SpawnActorfromClass "/Game/AI/Monster/DayMonster/Orc/BP/BP_EventOrc.BP_EventOrc_C" (Math|Conversions|ToTransform(Vector) _randomlocation) "AdjustIfPossibleButAlwaysSpawn" 0 0))
      (Utilities|Array|Add (Variables|Default|GetMonsterContainer) _returnvalue_2))))

(event Collision|EventActorBeginOverlap
  (params (OtherActor :type Actor%20Object%20Reference)))

(event EventTick
  (params (DeltaSeconds :type Float%20%28single-precision%29)))

(fn ConstructionScript)

(fn TraponPlayer
  (params (PlayerActor :type Actor%20Object%20Reference))
  (if (not (Variables|Default|GetIsOnce))
    (Variables|Default|SetIsOnce true)
    (bind _asbp_my_character_child (Utilities|Casting|CastToBP_MyCharacter_Child PlayerActor))
    (for _array_element (Variables|Default|GetMonsterContainer)
      (bind _asmy_aicontroller (Utilities|Casting|CastToMyAIController (Pawn|GetController _array_element)))
      (Variables|/Script/TeamAI.MyAIController|SetAIData _asmy_aicontroller (Utilities|Struct|MakeAIDataStruct (.walkspeed (Variables|/Script/TeamAI.MyAIController|GetAIData _asmy_aicontroller)) (.runspeed (Variables|/Script/TeamAI.MyAIController|GetAIData _asmy_aicontroller)) (.patrolrange (Variables|/Script/TeamAI.MyAIController|GetAIData _asmy_aicontroller)) (.attackrange (Variables|/Script/TeamAI.MyAIController|GetAIData _asmy_aicontroller)) (.attackcooltime (Variables|/Script/TeamAI.MyAIController|GetAIData _asmy_aicontroller)) 5e+03 6e+03 1.2e+02 (.hearingrange (Variables|/Script/TeamAI.MyAIController|GetAIData _asmy_aicontroller)) (.perceptionage (Variables|/Script/TeamAI.MyAIController|GetAIData _asmy_aicontroller))))
      (Class|MyAIController|SetAIState _asmy_aicontroller "State_BattleReady")
      (bind (_array_element_2 _array_index) (Utilities|Array|ForEachLoopwithBreak (Variables|/Script/TeamAI.MyAIController|GetAIBattleStateList _asmy_aicontroller) :!label _label)
        (:LoopBody
          (if (Utilities|Enum|Equal(Enum) _array_element_2 "Battle_Boundary")
            (Utilities|Array|RemoveIndex (Variables|/Script/TeamAI.MyAIController|GetAIBattleStateList _asmy_aicontroller) _array_index)
            (goto _label Break)))
        (:Completed
          (AI|Components|Blackboard|SetValueasObject (AI|GetBlackboard _asmy_aicontroller) (Utilities|Name|MakeLiteralName "TargetActor") _asbp_my_character_child)
          (AI|Logic|StartLogic (Variables|/Script/AIModule.AIController|GetBrainComponent _asmy_aicontroller)))))))
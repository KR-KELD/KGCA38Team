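; Battle room actor that runs a multi-round monster encounter behind cell doors.
; BeginPlay pre-spawns a pool of event orcs, opens the first cell door and places them at random navigable points with AI stopped.
; A player entering the box slides the room door on Tick and activates orc AI through the blackboard.
; Clearing a wave starts a timer that opens the next cell, reusing the orcs, then spawning a Cyclops and Troll.
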(event OnComponentBeginOverlap(Box)
  (params (OverlappedComponent :type Primitive%20Component%20Object%20Reference) (OtherActor :type Actor%20Object%20Reference) (OtherComp :type Primitive%20Component%20Object%20Reference) (OtherBodyIndex :type Integer) (bFromSweep :type Boolean) (SweepResult :type Hit%20Result%20Structure%20%28by%20ref%29))
  (if (not (Variables|Default|GetIsOnce))
    (if (Actor|ActorHasTag OtherActor "Player")
      (Variables|Default|SetBaBool true)
      (Variables|Default|SetIsOnce true)
      (CallFunction|RecognizePlayer OtherActor))))

(event Custom|AddDeadCount
  (params (String :type String))
  (bind _output_get (Variables|Default|SetMonsterCount (- (Variables|Default|GetMonsterCount) 1)))
  (if (<= _output_get 0)
    (Variables|Default|SetRound (+ (Variables|Default|GetRound) 1))
    (Variables|Default|SetMonsterCount (Utilities|Array|Length (Variables|Default|GetMonsterContainer)))
    (bind _returnvalue (Utilities|Time|SetTimerbyEvent (delegate Custom|RoundCooldown) 7.0))
    (Variables|Default|SetTimer _returnvalue)))

(event Custom|RoundCooldown
  (if (Variables|Default|GetLVCount)
    (bind _asbp_cell_door (Utilities|Casting|CastToBP_Cell_Door (Variables|Default|GetLV2)))
    (Variables|/MazeRunnerMapToolPlugins/MedievalDungeon/Blueprints/BP_Cell_Door.BP_Cell_Door_C|SetRotationBool _asbp_cell_door true)
    (CallFunction|RoundChange)
    (Utilities|Time|ClearandInvalidateTimerbyHandle (Variables|Default|GetTimer))
    (else
      (Variables|Default|SetLVCount true)
      (bind _asbp_cell_door_2 (Utilities|Casting|CastToBP_Cell_Door (Variables|Default|GetLV1)))
      (Variables|/MazeRunnerMapToolPlugins/MedievalDungeon/Blueprints/BP_Cell_Door.BP_Cell_Door_C|SetRotationBool _asbp_cell_door_2 true)
      (CallFunction|RoundChange)
      (Utilities|Time|ClearandInvalidateTimerbyHandle (Variables|Default|GetTimer)))))

(event EventBeginPlay
  (bind _output_get (Variables|Default|SetMonsterCount 10))
  ;[1 1 1] 갯수만큼 미리 만들어둠
  (CallFunction|MakeEventMonster _output_get)
  (bind _asbp_cell_door (Utilities|Casting|CastToBP_Cell_Door (Variables|Default|GetLV0)))
  (Variables|/MazeRunnerMapToolPlugins/MedievalDungeon/Blueprints/BP_Cell_Door.BP_Cell_Door_C|SetRotationBool _asbp_cell_door true)
  (CallFunction|RespawnEventMonster (Utilities|Array|Get(acopy) (Variables|Default|GetRespawnPoints)) 1e+03))

(event Collision|EventActorBeginOverlap
  (params (OtherActor :type Actor%20Object%20Reference)))

(event EventTick
  (params (DeltaSeconds :type Float%20%28single-precision%29))
  (bind _battleroomdoor (Variables|Default|GetBattleRoomDoor))
  (bind _rootcomponent (Variables|/Script/Engine.Actor|GetRootComponent _battleroomdoor))
  (bind _rootcomponent_2 (Variables|/Script/Engine.Actor|GetRootComponent _battleroomdoor))
  (bind _returnvalue (Transformation|GetWorldLocation _rootcomponent_2))
  (bind _returnvalue_2 (Transformation|GetWorldLocation _rootcomponent))
  (bind (_x _y _z) (Math|Vector|BreakVector _returnvalue_2))
  (bind (_x_2 _y_2 _z_2) (Math|Vector|BreakVector _returnvalue))
  (if (Variables|Default|GetBaBool)
    (Transformation|SetWorldLocation _rootcomponent_2 (Math|Vector|MakeVector _x_2 (Math|Interpolation|FInterpTo _y_2 5265.0 (Utilities|Time|GetWorldDeltaSeconds) 1e+01) _z_2) true false)
    (else
      (Transformation|SetWorldLocation _rootcomponent (Math|Vector|MakeVector _x (Math|Interpolation|FInterpTo _y 6605.0 (Utilities|Time|GetWorldDeltaSeconds) 1e+01) _z) true false))))

(fn ConstructionScript)

(fn MakeEventMonster
  (params (MonsterNumber :type Integer))
  (for _index (range 1 MonsterNumber)
    (bind _returnvalue (Game|SpawnActorfromClass "/Game/AI/Monster/DayMonster/Orc/BP/BP_EventOrc.BP_EventOrc_C" (Math|Conversions|ToTransform(Vector) (Math|Vector|VectorZero)) "AdjustIfPossibleButAlwaysSpawn" 0 0))
    (EventDispatchers|BindEventtoDeadDelegate _returnvalue (EventDispatchers|CreateEvent :!event Custom|AddDeadCount))
    (bind _asmy_aicontroller (Utilities|Casting|CastToMyAIController (Pawn|GetController _returnvalue)))
    (Variables|/Script/TeamAI.MyAIController|SetAIData _asmy_aicontroller (Utilities|Struct|MakeAIDataStruct (.walkspeed (Variables|/Script/TeamAI.MyAIController|GetAIData _asmy_aicontroller)) (.runspeed (Variables|/Script/TeamAI.MyAIController|GetAIData _asmy_aicontroller)) (.patrolrange (Variables|/Script/TeamAI.MyAIController|GetAIData _asmy_aicontroller)) (.attackrange (Variables|/Script/TeamAI.MyAIController|GetAIData _asmy_aicontroller)) (.attackcooltime (Variables|/Script/TeamAI.MyAIController|GetAIData _asmy_aicontroller)) 5e+03 6e+03 1.2e+02 (.hearingrange (Variables|/Script/TeamAI.MyAIController|GetAIData _asmy_aicontroller)) (.perceptionage (Variables|/Script/TeamAI.MyAIController|GetAIData _asmy_aicontroller))))
    (Utilities|Array|Add (Variables|Default|GetMonsterContainer) _returnvalue)
    (Class|AIBase|SetActorActive _returnvalue false)))

(fn RespawnEventMonster
  (params (RespawnPos :type Vector) (Radius :type Float%20%28single-precision%29))
  (bind _returnvalue (Transformation|GetActorLocation))
  (bind _returnvalue_2 (+ RespawnPos _returnvalue))
  (bind (_randomlocation _returnvalue_3) (AI|Navigation|GetRandomReachablePointinRadius _returnvalue_2 1e+03 0 0))
  (for _array_element (Variables|Default|GetMonsterContainer)
    (if _returnvalue_3
      (Class|AIBase|AIRespawn _array_element)
      (Transformation|SetActorLocation _array_element (+ _randomlocation "0, 0,200.000000") false false)
      (bind _asmy_aicontroller (Utilities|Casting|CastToMyAIController (Pawn|GetController _array_element)))
      (AI|Logic|StopLogic (Variables|/Script/AIModule.AIController|GetBrainComponent _asmy_aicontroller) "Start"))))

(fn RecognizePlayer
  (params (Player :type Actor%20Object%20Reference))
  (for _array_element (Variables|Default|GetMonsterContainer)
    (if (Variables|/Script/TeamAI.AIBase|GetIsAIActive _array_element)
      (bind _asmy_aicontroller (Utilities|Casting|CastToMyAIController (Pawn|GetController _array_element)))
      (Utilities|IsValid Player
        (:Is%20Valid
          (AI|Components|Blackboard|SetValueasObject (AI|GetBlackboard _asmy_aicontroller) (Utilities|Name|MakeLiteralName "TargetActor") Player))
        (:Is%20Not%20Valid
          _))
      (Class|MyAIController|UpdateState _asmy_aicontroller "State_BattleReady")
      (AI|Logic|StartLogic (Variables|/Script/AIModule.AIController|GetBrainComponent _asmy_aicontroller)))))

(fn RoundChange
  (bind _returnvalue (Transformation|GetActorLocation))
  (bind _respawnpoints (Variables|Default|GetRespawnPoints))
  (bind _output (Utilities|Array|Get(acopy) _respawnpoints 2))
  (bind _returnvalue_2 (+ _output _returnvalue))
  (switch int (Variables|Default|GetRound)
    (:2
      (CallFunction|RespawnEventMonster (Utilities|Array|Get(acopy) _respawnpoints 1) 1e+03)
      (CallFunction|RecognizePlayer))
    (:3
      (Utilities|FlowControl|Sequence
        (:then_0
          (bind _returnvalue_3 (Game|SpawnActorfromClass "/Game/AI/Monster/NightMonster/Cyclops/BP/BP_Cyclops.BP_Cyclops_C" (Math|Transform|MakeTransform (+ _returnvalue_2 "0,300.000000, 0") "0,180.000000, 0" "1,1,1") "AdjustIfPossibleButAlwaysSpawn" 0 0))
          (bind _asmy_aicontroller (Utilities|Casting|CastToMyAIController (Pawn|GetController _returnvalue_3)))
          (Class|MyAIController|SetAIState _asmy_aicontroller "State_Idle"))
        (:then_1
          (bind _returnvalue_4 (Game|SpawnActorfromClass "/Game/AI/Monster/DayMonster/Troll/BP/BP_Troll.BP_Troll_C" (Math|Transform|MakeTransform (+ _returnvalue_2 "0,-300.000000, 0") "0,180.000000, 0" "1,1,1") "AdjustIfPossibleButAlwaysSpawn" 0 0))
          (bind _asmy_aicontroller_2 (Utilities|Casting|CastToMyAIController (Pawn|GetController _returnvalue_4)))
          (Class|MyAIController|SetAIState _asmy_aicontroller_2 "State_Idle"))))))